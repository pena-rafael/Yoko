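; Neutral NPC Blueprint with empty attack, lock-on and BeginPlay events, so its event graph does nothing at runtime.
; SendTargetLocation writes the actor's location to Zone_GI's TargetPosition, and DistanceFromPlayerCheck returns its distance to the player.
; Disconnected leftovers hold an attack flag with debug print, a visibility toggle, and a timer call for SendTargetLocation gated on Vivo.
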(event Custom|Ataque)

(event EventTargetLockon)

(event EventBeginPlay)

(fn ConstructionScript)

(fn SendTargetLocation
  (bind _aszone_gi (Utilities|Casting|CastToZone_GI (Game|GetGameInstance)))
  (Variables|/Game/NPC/npc_inimigo/Zone_GI.Zone_GI_C|SetTargetPosition _aszone_gi (Transformation|GetActorLocation)))

(fn DistancefromPlayerCheck
  (return (Transformation|GetDistanceTo (Game|GetPlayerCharacter 0))))