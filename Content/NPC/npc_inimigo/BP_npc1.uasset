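; BP_npc1 is an enemy NPC that can be lock-on targeted and reports its position to the game instance.
; On BeginPlay, if alive, it sets a one-shot timer that writes its location to TargetPosition in Zone_GI.
; TargetLockon toggles the TargetVisual marker with a FlipFlop, and a helper returns distance to the player.
; The attack event is a stub that sets Atacando and prints debug text.
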(event Custom|Ataque
  (Variables|Default|SetAtacando true)
  (Development|PrintText "Hello"))

(event EventTargetLockon
  (bind _targetvisual (Variables|Default|GetTargetVisual))
  (Utilities|FlowControl|FlipFlop
    (:A
      (Development|SetHiddeninGame _targetvisual false false))
    (:B
      (Development|SetHiddeninGame _targetvisual true false))))

(event EventBeginPlay
  (if (Variables|Default|GetVivo)
    (Utilities|FlowControl|DoOnce false
      (:Completed
        (Utilities|Time|SetTimerbyFunctionName 0 "SendTargetLocation" 0.05)))))

(fn ConstructionScript)

(fn SendTargetLocation
  (bind _aszone_gi (Utilities|Casting|CastToZone_GI (Game|GetGameInstance)))
  (Variables|/Game/NPC/npc_inimigo/Zone_GI.Zone_GI_C|SetTargetPosition _aszone_gi (Transformation|GetActorLocation)))

(fn DistancefromPlayerCheck
  (return (Transformation|GetDistanceTo (Game|GetPlayerCharacter 0))))