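; Enemy NPC Blueprint that handles a basic attack state, a lock-on marker and distance checks against the player.
; Shortly after BeginPlay, if alive, a one-shot timer writes its location to the Zone_GI game instance as the target position.
; Ataque flags attacking and, early in the combo count, pulses the attack index for a second; combo-tracking nodes are unwired.
; TargetLockon uses a FlipFlop to toggle the target marker's visibility.
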(event Custom|Ataque
  (Variables|Default|SetAtacando true)
  (if (<= (Variables|Default|GetNCombo) 1)
    (Variables|Default|SetNAtaque 1)
    (Utilities|FlowControl|Delay 1.0)
    (Variables|Default|SetNAtaque 0)))

(event EventTargetLockon
  (bind _targetvisual (Variables|Default|GetTargetVisual))
  (Utilities|FlowControl|FlipFlop
    (:A
      (Development|SetHiddeninGame _targetvisual false false))
    (:B
      (Development|SetHiddeninGame _targetvisual true false))))

(event EventBeginPlay
  (if (Variables|Default|GetVivo)
    (Utilities|FlowControl|DoOnce false
      (:Completed
        (Utilities|Time|SetTimerbyFunctionName 0 "SendTargetLocation" 0.05)))))

(event EventTick
  (params (DeltaSeconds :type Float%20%28single-precision%29)))

(fn ConstructionScript)

(fn SendTargetLocation
  (bind _aszone_gi (Utilities|Casting|CastToZone_GI (Game|GetGameInstance)))
  (Variables|/Game/NPC/npc_inimigo/Zone_GI.Zone_GI_C|SetTargetPosition _aszone_gi (Transformation|GetActorLocation)))

(fn DistancefromPlayerCheck
  (return (Transformation|GetDistanceTo (Game|GetPlayerCharacter 0))))